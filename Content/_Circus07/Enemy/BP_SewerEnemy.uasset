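; Sewer chase enemy that crawls straight at the player and is killed by being stared down.
; Each Tick it uses view dot products to accelerate while the player's back is turned, scaling crawl audio with speed, otherwise resetting to base speed.
; Standing nearly still while facing it fills a timer that fires a death dispatcher, effects and destruction.
; Touching the player deals damage through the GameInstance, opening the sewer chase level when ModifyHP returns true.
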(event `self.ReceiveBeginPlay`
  (set `self.CurrentMoveSpeed` (`self.BaseMoveSpeed`))
  (set `CharacterMovementComponent.MaxWalkSpeed` (`self.CurrentMoveSpeed`) (`self.CharacterMovement`))
  (bind _asbp_first_person_character (cast `/Game/FirstPerson/Blueprints/BP_FirstPersonCharacter` (`GameplayStatics.GetPlayerCharacter` 0)))
  (set `self.CachedPlayerRef` _asbp_first_person_character)
  (set `PrimitiveComponent.bGenerateOverlapEvents` true (`self.CapsuleComponent`)))

(event `self.HitCollider.OnComponentBeginOverlap`
  (params (OverlappedComponent :type "PrimitiveComponent Object Reference") (OtherActor :type "Actor Object Reference") (OtherComp :type "PrimitiveComponent Object Reference") (OtherBodyIndex :type Integer) (bFromSweep :type Boolean) (SweepResult :type "HitResult Structure (by ref)"))
  (if (`self.bAlive`)
    (if (`self.ActorHasTag` OtherActor "Player")
      (bind _asbp_game_instance_main (cast `/Game/_Circus07/Blueprints/GameInstance/BP_GameInstanceMain` (`GameplayStatics.GetGameInstance`)))
      (bind _bisdead (`/Game/_Circus07/Blueprints/GameInstance/BP_GameInstanceMain.ModifyHP` _asbp_game_instance_main -100))
      (if _bisdead
        (`GameplayStatics.OpenLevel` "Lvl_03_SewerChase")))))

(event `self.ReceiveTick`
  (params (DeltaSeconds :type "Float (single-precision)"))
  (bind _cachedplayerref (`self.CachedPlayerRef`))
  (bind _returnvalue (`KismetMathLibrary.FClamp` (`KismetMathLibrary.NormalizeToRange` (`self.CurrentMoveSpeed`) (`self.BaseMoveSpeed`) (`self.MaxChaseSpeed`))))
  (bind _returnvalue_2 (`KismetMathLibrary.FClamp` (`KismetMathLibrary.NormalizeToRange` (`self.CurrentMoveSpeed`) (`self.BaseMoveSpeed`) (`self.MaxChaseSpeed`))))
  (set `self.DeltaT` DeltaSeconds)
  (if (`self.bAlive`)
    (`/Engine/EditorBlueprintResources/StandardMacros.IsValid` (`self.CachedPlayerRef`)
      (:`Is Valid`
        (if (< (`KismetMathLibrary.Dot_VectorVector` (`self.GetActorForwardVector` (`self.CachedPlayerRef`)) (`KismetMathLibrary.Normal` (- (`self.K2_GetActorLocation`) (`self.K2_GetActorLocation` (`self.CachedPlayerRef`))))) (`self.BackDotThreshold`))
          (`KismetSystemLibrary.PrintString` "Speeding Up")
          (set `self.CurrentMoveSpeed` (`KismetMathLibrary.FClamp` (+ (`self.CurrentMoveSpeed`) (* (`self.SpeedIncreaseRate`) (`self.DeltaT`))) (`self.BaseMoveSpeed`) (`self.MaxChaseSpeed`)))
          (set `CharacterMovementComponent.MaxWalkSpeed` (`self.CurrentMoveSpeed`) (`self.CharacterMovement`))
          (`AudioComponent.SetPitchMultiplier` (`self.CrawlAudio`) (`KismetMathLibrary.Lerp` 0.6 1.0 _returnvalue_2))
          (`AudioComponent.SetVolumeMultiplier` (`self.CrawlAudio`) (`KismetMathLibrary.Lerp` 0.35 0.8 _returnvalue_2))
          (else
            (`KismetSystemLibrary.PrintString` "Normal Speed")
            (set `self.CurrentMoveSpeed` (`self.BaseMoveSpeed`))
            (set `CharacterMovementComponent.MaxWalkSpeed` (`self.CurrentMoveSpeed`) (`self.CharacterMovement`))
            (set `AudioComponent.PitchMultiplier` (`KismetMathLibrary.Lerp` 1.0 2.0 _returnvalue) (`self.CrawlAudio`))
            (set `AudioComponent.VolumeMultiplier` (`KismetMathLibrary.Lerp` 0.35 1.0 _returnvalue) (`self.CrawlAudio`))))
        (`self.AddMovementInput` (`KismetMathLibrary.Normal` (- (`self.K2_GetActorLocation` _cachedplayerref) (`self.K2_GetActorLocation`))))
        (if (and (< (`KismetMathLibrary.VSizeXY` (`self.GetVelocity` _cachedplayerref)) (`self.StillSpeedThreshold`)) (> (`KismetMathLibrary.Dot_VectorVector` (`self.GetActorForwardVector` _cachedplayerref) (`KismetMathLibrary.Normal` (- (`self.K2_GetActorLocation`) (`self.K2_GetActorLocation` (`self.CachedPlayerRef`))))) (`self.FacingDotThreshold`)))
          (bind _output_get (set `self.FacingTimer` (+ (`self.FacingTimer`) (`self.DeltaT`))))
          (if (>= _output_get (`self.KillTimeRequired`))
            (`self.OnEnemyKilled`))
          (else
            (set `self.FacingTimer` 0.0)))))))

(event `OnEnemyKilled`
  (set `self.bAlive` false)
  (`self.OnEnemyKilledDispatcher`)
  (`AudioComponent.FadeOut` (`self.CrawlAudio`) 0.3 0.0 "Linear")
  (`|ExecutionSequence`
    (:`then_0`
      (`GameplayStatics.SpawnEmitterAtLocation` "/Engine/Tutorial/SubEditors/TutorialAssets/TutorialParticleSystem.TutorialParticleSystem" (`self.K2_GetActorLocation`)))
    (:`then_1`
      (`GameplayStatics.PlaySoundAtLocation` "/Game/_Circus07/Sound_Effects/One_Time/Bell.Bell" (`self.K2_GetActorLocation`) (struct) 1.0 1.0 0.0 null null null null))
    (:`then_2`
      (`self.K2_DestroyActor`))))

(fn `UserConstructionScript`)