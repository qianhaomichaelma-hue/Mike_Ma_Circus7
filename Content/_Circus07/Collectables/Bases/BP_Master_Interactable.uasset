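; Master collectable actor for pickups, the parent class that defines collection rules per collectable type.
; On sphere overlap with the first-person character, it checks whether that type can be collected (health or shield below max, essentials always) and refreshes the character's UI.
; A successful pickup broadcasts OnInteracted with type and point value to the Level Blueprint, then destroys itself.
; The construction script tints the mesh through a dynamic material instance.
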(event `self.CollisionSphere.OnComponentBeginOverlap`
  (params (OverlappedComponent :type "PrimitiveComponent Object Reference") (OtherActor :type "Actor Object Reference") (OtherComp :type "PrimitiveComponent Object Reference") (OtherBodyIndex :type Integer) (bFromSweep :type Boolean) (SweepResult :type "HitResult Structure (by ref)"))
  (bind _asbp_first_person_character (cast `/Game/FirstPerson/Blueprints/BP_FirstPersonCharacter` OtherActor))
  (bind _canbepickedup (`self.CanBePickedUp` _asbp_first_person_character))
  (if _canbepickedup
    (`self.OnPickup` _asbp_first_person_character))
  (`/Game/FirstPerson/Blueprints/BP_FirstPersonCharacter.RefreshUI` _asbp_first_person_character))

(event `OnPickup`
  (params (Character :type "/Game/FirstPerson/Blueprints/BP_FirstPersonCharacter Object Reference"))
  ; 有东西被捡起的时候，触发这个Event Dispatchers（发送信号），并传递至关卡蓝图
  (`self.OnInteracted` (`self.CollectableType`) (`self.PointValue`))
  (`self.K2_DestroyActor`))

(fn `CanBePickedUp`
  (params (Character :type "/Game/FirstPerson/Blueprints/BP_FirstPersonCharacter Object Reference"))
  (returns (CanBePickedUp :type Boolean))
  ; 使用一个Enum定义一共有哪些可收集物，并在父类蓝图中定义收集条件，便于项目的后续扩展
  (switch `/Game/_Circus07/Collectables/Enum/E_CollectableType` (`self.CollectableType`)
    (:`NewEnumerator0`
      (return (< (`/Game/FirstPerson/Blueprints/BP_FirstPersonCharacter.CurrentHealth` Character) (`/Game/FirstPerson/Blueprints/BP_FirstPersonCharacter.MaxHealth` Character))))
    (:`NewEnumerator1`
      (return (< (`/Game/FirstPerson/Blueprints/BP_FirstPersonCharacter.CurrentShield` Character) (`/Game/FirstPerson/Blueprints/BP_FirstPersonCharacter.MaxShield` Character))))
    (:`NewEnumerator2`
      (return true))))

(fn `UserConstructionScript`
  (bind _returnvalue (`PrimitiveComponent.CreateDynamicMaterialInstance` (`self.StaticMesh`) 0 "/Game/_Circus07/Collectables/Assets/Materials/M_Collectable_Inst.M_Collectable_Inst" "None"))
  (bind _output_get (set `self.Material` _returnvalue))
  (`MaterialInstanceDynamic.SetVectorParameterValue` _output_get "Color" (`self.Color`)))