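; BP_BaseHealth is a base collectable that restores health to the character who picks it up.
; On pickup it adds HealthToAdd to the character's CurrentHealth, clamped between zero and MaxHealth, then calls the parent pickup logic.
; Its CanBePickedUp override calls the parent but ignores that result, refusing pickup only when the character's health equals MaxHealth.
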(event `self.OnPickup`
  (params (Character :type "/Game/FirstPerson/Blueprints/BP_FirstPersonCharacter Object Reference"))
  (set `/Game/FirstPerson/Blueprints/BP_FirstPersonCharacter.CurrentHealth` (`KismetMathLibrary.FClamp` (+ (`/Game/FirstPerson/Blueprints/BP_FirstPersonCharacter.CurrentHealth` Character) (`self.HealthToAdd`)) 0.0 (`/Game/FirstPerson/Blueprints/BP_FirstPersonCharacter.MaxHealth` Character)) Character)
  (`parent.OnPickup` Character))

(fn `CanBePickedUp`
  (params (Character :type "/Game/FirstPerson/Blueprints/BP_FirstPersonCharacter Object Reference"))
  (returns (CanBePickedUp :type Boolean))
  (`parent.CanBePickedUp` Character)
  (if (== (`/Game/FirstPerson/Blueprints/BP_FirstPersonCharacter.MaxHealth` Character) (`/Game/FirstPerson/Blueprints/BP_FirstPersonCharacter.CurrentHealth` Character))
    (return false)
    (else
      (return true))))

(fn `UserConstructionScript`
  (`parent.UserConstructionScript`))