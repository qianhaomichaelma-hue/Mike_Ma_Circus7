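; BP_BaseShield is a base collectable Blueprint that adds shield to the character who picks it up.
; On pickup it adds ShieldToAdd to the character's CurrentShield, then runs the parent pickup logic.
; CanBePickedUp calls the parent but ignores its result, refusing pickup whenever the full amount would push the shield above MaxShield, so partial top-ups never happen.
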(event `self.OnPickup`
  (params (Character :type "/Game/FirstPerson/Blueprints/BP_FirstPersonCharacter Object Reference"))
  (set `/Game/FirstPerson/Blueprints/BP_FirstPersonCharacter.CurrentShield` (+ (`/Game/FirstPerson/Blueprints/BP_FirstPersonCharacter.CurrentShield` Character) (`self.ShieldToAdd`)) Character)
  (`parent.OnPickup` Character))

(fn `CanBePickedUp`
  (params (Character :type "/Game/FirstPerson/Blueprints/BP_FirstPersonCharacter Object Reference"))
  (returns (CanBePickedUp :type Boolean))
  (`parent.CanBePickedUp` Character)
  (if (> (+ (`/Game/FirstPerson/Blueprints/BP_FirstPersonCharacter.CurrentShield` Character) (`self.ShieldToAdd`)) (`/Game/FirstPerson/Blueprints/BP_FirstPersonCharacter.MaxShield` Character))
    (return false)
    (else
      (return true))))

(fn `UserConstructionScript`
  (`parent.UserConstructionScript`))