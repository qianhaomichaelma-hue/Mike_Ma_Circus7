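; Base Blueprint for collectable pickups that the first-person player collects by walking into them.
; A sphere overlap with BP_FirstPersonCharacter checks CanBePickedUp, which returns true here, then runs OnPickup.
; OnPickup plays an optional sound at the mesh location and destroys the actor.
; The construction script gives the mesh a dynamic collectable material tinted by the Color variable.
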(event `self.CollisionSphere.OnComponentBeginOverlap`
  (params (OverlappedComponent :type "PrimitiveComponent Object Reference") (OtherActor :type "Actor Object Reference") (OtherComp :type "PrimitiveComponent Object Reference") (OtherBodyIndex :type Integer) (bFromSweep :type Boolean) (SweepResult :type "HitResult Structure (by ref)"))
  (bind _asbp_first_person_character (cast `/Game/FirstPerson/Blueprints/BP_FirstPersonCharacter` OtherActor))
  (`self.OnPlayerOverlap` _asbp_first_person_character))

(event `OnPlayerOverlap`
  (params (Character :type "/Game/FirstPerson/Blueprints/BP_FirstPersonCharacter Object Reference"))
  (bind _canbepickedup (`self.CanBePickedUp` Character))
  (if _canbepickedup
    (`self.OnPickup` Character)))

(event `OnPickup`
  (params (Character :type "/Game/FirstPerson/Blueprints/BP_FirstPersonCharacter Object Reference"))
  (bind _pickupsound (`self.PickupSound`)
    (:`then`
      (`GameplayStatics.PlaySoundAtLocation` _pickupsound (`SceneComponent.K2_GetComponentLocation` (`self.StaticMesh`)) (struct) 1.0 1.0 0.0 null null null null))
    (:`else`
      _))
  (`self.K2_DestroyActor`))

(fn `CanBePickedUp`
  (params (Character :type "/Game/FirstPerson/Blueprints/BP_FirstPersonCharacter Object Reference"))
  (returns (CanBePickedUp :type Boolean))
  (return true))

(fn `UserConstructionScript`
  (bind _returnvalue (`PrimitiveComponent.CreateDynamicMaterialInstance` (`self.StaticMesh`) 0 "/Game/_Circus07/Collectables/Assets/Materials/M_Collectable_Inst.M_Collectable_Inst" "None"))
  (bind _output_get (set `self.Material` _returnvalue))
  (`MaterialInstanceDynamic.SetVectorParameterValue` _output_get "Color" (`self.Color`)))