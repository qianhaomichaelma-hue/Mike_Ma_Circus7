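; Interactable light switch that turns its point light on and off.
; OnInteract checks a boolean on-state, flips it and sets the light's visibility to match.
; ShowFocus and HideFocus show and hide a widget that serves as the focus indicator.
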(event `/Game/_Circus07/Blueprints/BPI/BPI_Interactble.OnInteract`
  (if (`self.BIsOn`)
    (`SceneComponent.SetVisibility` (`self.PointLight`) false false)
    (set `self.BIsOn` false)
    (else
      (`SceneComponent.SetVisibility` (`self.PointLight`) true false)
      (set `self.BIsOn` true))))

(event `/Game/_Circus07/Blueprints/BPI/BPI_Interactble.HideFocus`
  (`SceneComponent.SetVisibility` (`self.Widget`) false false))

(event `/Game/_Circus07/Blueprints/BPI/BPI_Interactble.ShowFocus`
  (`SceneComponent.SetVisibility` (`self.Widget`) true false))

(fn `UserConstructionScript`)