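; Game Instance Blueprint that holds player progress and state: completed levels, total score, collected items and player HP.
; Levels are recorded by name in a map with a debug print, and completion checks only test whether the key exists.
; Score accumulates additively, and collected item names are added without duplicates.
; HP changes are clamped between zero and the maximum, returning whether HP has run out.
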(fn `AddCollectedItem`
  (params (ItemName :type String))
  (if (not (`KismetArrayLibrary.Array_Contains` (`self.CollectedItems`) ItemName))
    (`KismetArrayLibrary.Array_Add` (`self.CollectedItems`) ItemName)))

(fn `AddScore`
  (params (ScoreAmount :type Integer))
  (set `self.TotalScore` (+ ScoreAmount (`self.TotalScore`))))

(fn `IsLevelComplete`
  (params (LevelName :type String))
  (returns (`bIsComplete ` :type Boolean))
  (return (`BlueprintMapLibrary.Map_Contains` (`self.CompletedLevels`) LevelName)))

(fn `MarkLevelComplete`
  (params (LevelName :type String))
  (`BlueprintMapLibrary.Map_Add` (`self.CompletedLevels`) LevelName true)
  (`KismetSystemLibrary.PrintString` "\"Level Completed: \" + LevelName"))

(fn `ModifyHP`
  (params (Amount :type Integer))
  (returns (bIsDead :type Boolean))
  (bind _output_get (set `self.PlayerCurrentHP` (`KismetMathLibrary.Clamp` (+ Amount (`self.PlayerCurrentHP`)) 0 (`self.PlayerMaxHP`))))
  (return (<= _output_get 0)))