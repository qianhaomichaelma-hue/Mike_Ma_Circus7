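; BP_LevelPortal is an overlap-triggered portal that completes a level and travels to another.
; Overlapping its Box marks CompleteLevelName complete in BP_GameInstanceMain, prints a message, fades the camera out, waits briefly, then opens TargetLevel.
; The Player tag is checked only before the level opens, so any overlapping actor triggers completion and the fade.
; A BP_FashionShowGM completion call remains in the graph but never runs.
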(event `self.Box.OnComponentBeginOverlap`
  (params (OverlappedComponent :type "PrimitiveComponent Object Reference") (OtherActor :type "Actor Object Reference") (OtherComp :type "PrimitiveComponent Object Reference") (OtherBodyIndex :type Integer) (bFromSweep :type Boolean) (SweepResult :type "HitResult Structure (by ref)"))
  ;[0.15 0.1094 0.04433 0.5] 0427 删改
  (bind _asbp_game_instance_main (cast `/Game/_Circus07/Blueprints/GameInstance/BP_GameInstanceMain` (`GameplayStatics.GetGameInstance`)))
  (`/Game/_Circus07/Blueprints/GameInstance/BP_GameInstanceMain.MarkLevelComplete` _asbp_game_instance_main (`self.CompleteLevelName`))
  (`KismetSystemLibrary.PrintString` "Level Complete!")
  (`PlayerCameraManager.StartCameraFade` :`self` (`GameplayStatics.GetPlayerCameraManager` 0) :`ToAlpha` 1.0 :`Duration` 0.5)
  (`KismetSystemLibrary.Delay` 0.5)
  (if (`self.ActorHasTag` OtherActor "Player")
    (`GameplayStatics.OpenLevel` (`self.TargetLevel`))))

(fn `UserConstructionScript`)