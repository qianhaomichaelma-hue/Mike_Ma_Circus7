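; BP_TrafficLight is a signal light actor that displays the red or green light state held by the fashion show game mode.
; It caches BP_FashionShowGM on BeginPlay, then polls its IsRedLight, IsWarning and BlinkState flags every Tick to set SignalLight's color and intensity.
; During a warning the light flashes in the current color by following the game mode's BlinkState; otherwise it stays lit.
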(event `self.ReceiveBeginPlay`
  (bind _asbp_fashion_show_gm (cast `/Game/_Circus07/Blueprints/GameMode/BP_FashionShowGM` (`GameplayStatics.GetGameMode`)))
  (set `self.GameModeRef` _asbp_fashion_show_gm))

(event `self.ReceiveTick`
  (params (DeltaSeconds :type "Float (single-precision)"))
  (bind _signallight (`self.SignalLight`))
  (bind _signallight_2 (`self.SignalLight`))
  (bind _gamemoderef (`self.GameModeRef`))
  (`/Engine/EditorBlueprintResources/StandardMacros.IsValid` _gamemoderef
    (:`Is Valid`
      (if (`/Game/_Circus07/Blueprints/GameMode/BP_FashionShowGM.bIsWarning` _gamemoderef)
        (if (`/Game/_Circus07/Blueprints/GameMode/BP_FashionShowGM.bBlinkState` _gamemoderef)
          (`LightComponent.SetIntensity` _signallight_2 50000.0)
          (if (`/Game/_Circus07/Blueprints/GameMode/BP_FashionShowGM.bIsRedLight` _gamemoderef)
            (`LightComponent.SetLightColor` _signallight (struct :`R` 1.0 :`G` 0.001029 :`B` 0.048803 :`A` 1.0) true)
            (else
              (`LightComponent.SetLightColor` _signallight (struct :`R` 0.015101 :`G` 1.0 :`B` 0.047461 :`A` 1.0) true)))
          (else
            (`LightComponent.SetIntensity` _signallight_2 0.0)))
        (elif (`/Game/_Circus07/Blueprints/GameMode/BP_FashionShowGM.bIsRedLight` _gamemoderef)
          (`LightComponent.SetIntensity` _signallight_2 50000.0)
          (`LightComponent.SetLightColor` _signallight_2 (struct :`R` 1.0 :`G` 0.001029 :`B` 0.048803 :`A` 1.0) true)
          (else
            (`LightComponent.SetIntensity` _signallight_2 50000.0)
            (`LightComponent.SetLightColor` _signallight_2 (struct :`R` 0.015101 :`G` 1.0 :`B` 0.047461 :`A` 1.0) true)))))))

(fn `UserConstructionScript`)