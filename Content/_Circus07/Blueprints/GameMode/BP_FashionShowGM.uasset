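; Game mode for the Fashion Show level, running a red light, green light game that starts on BeginPlay and pauses the music on red.
; Randomly timed phases end in a warning of accelerating beeps before switching.
; On red, Tick compares the player's distance from their stop position to a threshold, then fades out and returns violators to the start.
; OnLevelComplete is empty; its completion and score logic is disconnected.
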(event `self.ReceiveBeginPlay`
  (`parent.ReceiveBeginPlay`)
  (bind _outactors (`GameplayStatics.GetAllActorsOfClass` "/Game/_Circus07/Blueprints/BP_FashionMusic.BP_FashionMusic_C"))
  (set `self.MusicSourceRef` (`|GetArrayItem` _outactors))
  (`self.StartGame`))

(event `self.ReceiveTick`
  (params (DeltaSeconds :type "Float (single-precision)"))
  (if (`self.bGameStarted`)
    (if (`self.bIsRedLight`)
      (if (not (`self.bIsRespawning`))
        (if (> (`KismetMathLibrary.Vector_Distance` (`self.K2_GetActorLocation` (`GameplayStatics.GetPlayerCharacter` 0)) (`self.PlayerStartLocation`)) (`self.MovementThreshold`))
          (`self.OnPlayerCaught`))))))

(event `StartGame`
  (`/Game/_Circus07/Blueprints/BP_FashionMusic.StartMusic` (`self.MusicSourceRef`))
  (set `self.bGameStarted` true)
  (set `self.RespawnPoint` (`self.K2_GetActorLocation` (`GameplayStatics.GetPlayerCharacter` 0)))
  (`self. SwitchToGreen`))

(event `OnPlayerCaught`
  (set `self.bIsRespawning` true)
  (`KismetSystemLibrary.PrintString` "CAUGHT! Returning to start..." true true (struct :`R` 1.0 :`B` 0.047378 :`A` 1.0))
  (`Controller.SetIgnoreMoveInput` (`GameplayStatics.GetPlayerController` 0) true)
  (`Controller.SetIgnoreLookInput` (`GameplayStatics.GetPlayerController` 0) true)
  (`PlayerCameraManager.StartCameraFade` :`self` (`GameplayStatics.GetPlayerCameraManager` 0) :`ToAlpha` 1.0 :`Duration` 0.35 :`bHoldWhenFinished` true)
  (`KismetSystemLibrary.Delay` 0.5)
  (`self.K2_SetActorLocation` (`GameplayStatics.GetPlayerCharacter` 0) (`self.RespawnPoint`) false false)
  (set `self.PlayerStartLocation` (`self.RespawnPoint`))
  (`PlayerCameraManager.StartCameraFade` :`self` (`GameplayStatics.GetPlayerCameraManager` 0) :`FromAlpha` 1.0 :`Duration` 0.35)
  (`KismetSystemLibrary.Delay` 0.2)
  (`Controller.SetIgnoreMoveInput` (`GameplayStatics.GetPlayerController` 0) false)
  (`Controller.SetIgnoreLookInput` (`GameplayStatics.GetPlayerController` 0) false)
  (set `self.bIsRespawning` false))

(event `SwitchToGreen`
  (`/Game/_Circus07/Blueprints/BP_FashionMusic.ResumeMusic` (`self.MusicSourceRef`))
  (set `self.bIsRedLight` false)
  (set `self.bIsWarning` false)
  (set `self.bBlinkState` true)
  (`KismetSystemLibrary.PrintString` "GREEN LIGHT - GO!" true true (struct :`R` 0.03061 :`G` 1.0 :`B` 0.118968 :`A` 1.0) 5.0)
  (`KismetSystemLibrary.K2_SetTimer` null "StartWarning" (`KismetMathLibrary.FMax` (- (`KismetMathLibrary.RandomFloatInRange` (`self.GreenLightDurationMin`) (`self.GreenLightDurationMax`)) (`self.WarningDuration`)) 0.1)))

(event `SwitchToRed`
  (`/Game/_Circus07/Blueprints/BP_FashionMusic.PauseMusic` (`self.MusicSourceRef`))
  (set `self.bIsRedLight` true)
  (set `self.bIsWarning` false)
  (set `self.bBlinkState` true)
  (`KismetSystemLibrary.PrintString` "RED LIGHT - STOP!" true true (struct :`R` 1.0 :`G` 0.081356 :`B` 0.36361 :`A` 1.0))
  (set `self.PlayerStartLocation` (`self.K2_GetActorLocation` (`GameplayStatics.GetPlayerCharacter` 0)))
  (`KismetSystemLibrary.K2_SetTimer` null "StartWarning" (`KismetMathLibrary.FMax` (- (`KismetMathLibrary.RandomFloatInRange` (`self.RedLightDurationMin`) (`self.RedLightDurationMax`)) (`self.WarningDuration`)) 0.1)))

(event `StartWarning`
  (set `self.bIsWarning` true)
  (set `self.CurrentBlinkInterval` 0.4)
  (`KismetSystemLibrary.PrintString` "⚠️ Warning - Light changing soon!" true true (struct :`R` 1.0 :`G` 0.865588 :`A` 1.0))
  (`self.DoBlink`))

(event `DoBlink`
  (set `self.bBlinkState` (not (`self.bBlinkState`)))
  (`GameplayStatics.PlaySoundAtLocation` "/Game/_Circus07/Sound_Effects/Beep2.Beep2" (0.0 0.0 0.0) (struct) 1.0 1.0 0.0 null null null null)
  (bind _output_get (set `self.CurrentBlinkInterval` (* (`self.CurrentBlinkInterval`) 0.5)))
  (if (> _output_get 0.05)
    (bind _returnvalue (`KismetSystemLibrary.K2_SetTimer` null "DoBlink" (`self.CurrentBlinkInterval`)))
    (set `self.BlinkTimerHandle` _returnvalue)
    (elif (`self.bIsRedLight`)
      (`self. SwitchToGreen`)
      (else
        (`self.SwitchToRed`)))))

(event `OnLevelComplete`)

(fn `UserConstructionScript`)